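; AI projectile actor that damages AI or player characters on overlap and destroys itself one second after BeginPlay.
; The ProjectileOverlap component's begin-overlap casts the other actor to AIChar_BP, requiring a capsule hit, then otherwise to PlayerChar_BP.
; Each branch uses DoOnce before ApplyDamage, with less damage for the player, then destroys the projectile.
; The AI branch's ApplyDamage has no DamagedActor connected, and debug prints remain throughout.
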(event OnComponentBeginOverlap(ProjectileOverlap)
  (params (OverlappedComponent :type Primitive%20Component%20Object%20Reference) (OtherActor :type Actor%20Object%20Reference) (OtherComp :type Primitive%20Component%20Object%20Reference) (OtherBodyIndex :type Integer) (bFromSweep :type Boolean) (SweepResult :type Hit%20Result%20Structure%20%28by%20ref%29))
  (bind _returnvalue (Components|GetOwner))
  (Development|PrintString "On Component Begin Overlap (Projectile)!!!!" true true "(R=0.000000,G=0.660000,B=1.000000,A=1.000000)" 122.0)
  (bind _asaichar_bp (Utilities|Casting|CastToAIChar_BP OtherActor)
    (:then
      (Development|PrintText "Cast success: I think I got hit!!!" true true "(R=1.000000,G=0.000000,B=0.203948,A=1.000000)" 111.0)
      (if (== OtherComp (Variables|/Script/Engine.Character|GetCapsuleComponent _asaichar_bp))
        (Utilities|FlowControl|DoOnce false
          (:Completed
            (Game|Damage|ApplyDamage 0 1e+01 0 _returnvalue)
            (Actor|DestroyActor :!label _label)))))
    (:CastFailed
      (bind _asplayer_char_bp (Utilities|Casting|CastToPlayerChar_BP OtherActor))
      (Utilities|FlowControl|DoOnce false
        (:Completed
          (Development|PrintText "after Cast to player_BP, to apply damage?" true true "(R=0.896785,G=1.000000,B=0.844667,A=1.000000)" 1.2e+05)
          (Game|Damage|ApplyDamage _asplayer_char_bp 5.0 0 _returnvalue)
          (goto _label))))))

(event EventBeginPlay
  (Utilities|FlowControl|Delay 1.0)
  (Actor|DestroyActor)
  (Development|PrintText "Begin B-Play"))

(fn ConstructionScript)