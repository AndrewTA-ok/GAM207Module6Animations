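; AI controller Blueprint that runs the AI_BT behavior tree and tracks a perceived enemy.
; AI Perception updates accept AIChar_BP or PlayerChar_BP actors, storing a sensed one as TargetEnemy in the blackboard.
; A failed sense clears TargetEnemy without checking which actor was lost.
; SetFocus is called on sensing with no actor supplied, and debug prints trace each step.
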(event OnTargetPerceptionUpdated(AIPerception)
  (params (Actor :type Actor%20Object%20Reference) (Stimulus :type AI%20Stimulus%20Structure))
  (bind _returnvalue (AI|GetBlackboard 0))
  (bind _returnvalue_2 (Utilities|Name|MakeLiteralName "TargetEnemy"))
  (Development|PrintString "On target: AI perception" true true "(R=0.005633,G=0.103894,B=0.154514,A=1.000000)" 1111.0)
  (Utilities|Casting|CastToAIChar_BP Actor
    (:then
      _)
    (:CastFailed
      (Utilities|Casting|CastToPlayerChar_BP Actor)))
  (if (.bSuccessfullySensed (Utilities|Struct|BreakAIStimulus Stimulus))
    (bind _output_get (Variables|Default|SetTargetEnemy Actor))
    (Utilities|IsValid _returnvalue
      (:Is%20Valid
        (Development|PrintText "Valid" true true "(R=0.000000,G=0.660000,B=1.000000,A=1.000000)" 111.0)
        (AI|Components|Blackboard|SetValueasObject _returnvalue _returnvalue_2 _output_get)
        (AI|SetFocus)))
    (else
      (Variables|Default|SetTargetEnemy 0)
      (Development|PrintString "Set blank target" true true "(R=0.928353,G=0.966712,B=1.000000,A=1.000000)" 1125.0)
      (AI|Components|Blackboard|SetValueasObject _returnvalue _returnvalue_2 0))))

(event EventBeginPlay
  (Development|PrintString "Behavior Tree!for AICont!!" true true "(R=0.000000,G=0.660000,B=1.000000,A=1.000000)" 1e+01)
  (AI|RunBehaviorTree "/Game/AI/AI_BT.AI_BT"))

(fn ConstructionScript)